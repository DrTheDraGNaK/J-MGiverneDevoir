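; Enemy that detects the third-person player through AI perception and drives chase state in its Blackboard.
; Sensing the player stores it as TargetEnemy, sets InLightOffSite and cancels the pending lose-chase timer.
; Losing the player starts a ChaseLostDelay timer that clears only the flag, giving a grace period before chase ends.
; A looping random-wander routine using navmesh points and AIMoveTo exists but is never triggered in this graph.
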(event `self.ReceiveBeginPlay`)

(event `Move to random Pos`
  (bind (_randomlocation _returnvalue) (`NavigationSystemV1.K2_GetRandomLocationInNavigableRadius` (`self.K2_GetActorLocation`) 500.0 null null))
  (if _returnvalue
    (`|AIMoveTo` self _randomlocation null
      (:`OnSuccess`
        (`KismetSystemLibrary.PrintString` "Arrivé")
        (`self.Move to random Pos`)))
    (else
      (`KismetSystemLibrary.PrintString` "Failed to find path"))))

(event `self.AIPerception.OnTargetPerceptionUpdated`
  (params (Actor :type "Actor Object Reference") (Stimulus :type "AIStimulus Structure"))
  (bind _returnvalue (`AIBlueprintHelperLibrary.GetBlackboard` self))
  (bind _asthird_person_character (cast `/Game/ThirdPersonCPP/Blueprints/ThirdPersonCharacter` Actor))
  (if (`.bSuccessfullySensed` (break `AIStimulus` Stimulus))
    (`BlackboardComponent.SetValueAsObject` _returnvalue "TargetEnemy" _asthird_person_character)
    (`BlackboardComponent.SetValueAsBool` _returnvalue "InLightOffSite" true)
    (`KismetSystemLibrary.K2_ClearAndInvalidateTimerHandle` (`self.CancelChaseTimer`))
    (else
      (bind _returnvalue_2 (`KismetSystemLibrary.K2_SetTimerDelegate` (delegate `CancelChase`) (`self.ChaseLostDelay`)))
      (set `self.CancelChaseTimer` _returnvalue_2))))

(event `CancelChase`
  (`BlackboardComponent.SetValueAsBool` (`AIBlueprintHelperLibrary.GetBlackboard` self) "InLightOffSite" false))

(fn `UserConstructionScript`)
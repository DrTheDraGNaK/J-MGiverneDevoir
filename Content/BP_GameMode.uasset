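; Game mode that owns the save system, restoring the player's level and position when play begins.
; BeginPlay reads the slot name from the LoadFromMenu game instance, then creates a save, opens the saved map, or restores the character transform if flagged.
; Events save the transform, load by restarting the level, delete the save and restart, or record a new map with position restore disabled, without opening it.
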(event `self.ReceiveBeginPlay`
  (bind _asload_from_menu (cast `/Game/LoadFromMenu` (`GameplayStatics.GetGameInstance`)))
  (set `self.Save File Name` (`/Game/LoadFromMenu.SaveFileName` _asload_from_menu))
  (bind _returnvalue (`GameplayStatics.DoesSaveGameExist` (`self.Save File Name`)))
  (if _returnvalue
    (bind _returnvalue_2 (`GameplayStatics.LoadGameFromSlot` (`self.Save File Name`)))
    (bind _asbp_save_game (cast `/Game/BP_SaveGame` _returnvalue_2))
    (set `self.SaveGameRef` _asbp_save_game)
    (bind _returnvalue_3 (`GameplayStatics.GetCurrentLevelName` true))
    (if (== (`KismetStringLibrary.Conv_StringToName` _returnvalue_3) (`/Game/BP_SaveGame.MapName` (`self.SaveGameRef`)))
      (if (`/Game/BP_SaveGame.UseSaveLocation` (`self.SaveGameRef`))
        (bind _asthird_person_character (cast `/Game/ThirdPersonCPP/Blueprints/ThirdPersonCharacter` (`GameplayStatics.GetPlayerCharacter` 0)))
        (`SceneComponent.K2_SetWorldTransform` (`Actor.RootComponent` _asthird_person_character) (`/Game/BP_SaveGame.CharTransform` (`self.SaveGameRef`)) false false))
      (else
        (`GameplayStatics.OpenLevel` (`/Game/BP_SaveGame.MapName` (`self.SaveGameRef`)))))
    (else
      (bind _returnvalue_4 (`GameplayStatics.CreateSaveGameObject` "/Game/BP_SaveGame.BP_SaveGame_C"))
      (bind _returnvalue_5 (`GameplayStatics.GetCurrentLevelName` true))
      (set `/Game/BP_SaveGame.MapName` (`KismetStringLibrary.Conv_StringToName` _returnvalue_5) _returnvalue_4)
      (`GameplayStatics.SaveGameToSlot` _returnvalue_4 (`self.Save File Name`)))))

(event `SaveGame`
  ;[1 1 1] SaveGame
  (bind _returnvalue (`GameplayStatics.LoadGameFromSlot` (`self.Save File Name`)))
  (bind _asbp_save_game (cast `/Game/BP_SaveGame` _returnvalue))
  (set `/Game/BP_SaveGame.CharTransform` (`self.GetTransform` (cast `/Game/ThirdPersonCPP/Blueprints/ThirdPersonCharacter` (`GameplayStatics.GetPlayerCharacter` 0) :!pure true)) _asbp_save_game)
  (set `/Game/BP_SaveGame.UseSaveLocation` true _asbp_save_game)
  (`GameplayStatics.SaveGameToSlot` _asbp_save_game (`self.Save File Name`)))

(event `LoadGame`
  ;[1 1 1] LoadGame
  (`KismetSystemLibrary.ExecuteConsoleCommand` "RestartLevel" null))

(event `RestartLevel`
  ;[1 1 1] delete/restart
  (`GameplayStatics.DeleteGameInSlot` (`self.Save File Name`))
  (`KismetSystemLibrary.ExecuteConsoleCommand` "RestartLevel" null))

(event `ChangeLevels`
  (params (MapName :type Name))
  ;[1 1 1] Change levels
  (bind _returnvalue (`GameplayStatics.LoadGameFromSlot` (`self.Save File Name`)))
  (bind _asbp_save_game (cast `/Game/BP_SaveGame` _returnvalue))
  (set `/Game/BP_SaveGame.UseSaveLocation` false _asbp_save_game)
  (set `/Game/BP_SaveGame.MapName` MapName _asbp_save_game)
  (`GameplayStatics.SaveGameToSlot` _asbp_save_game (`self.Save File Name`)))

(fn `UserConstructionScript`)